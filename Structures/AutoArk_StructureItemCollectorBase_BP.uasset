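; Base Blueprint for an item collector structure that periodically gathers nearby objects into an inventory.
; A looping timer started on BeginPlay runs a multi-sphere object trace from the structure's location.
; For each hit, it adds one item of the configured pickup archetype to the target inventory and destroys the hit actor, without checking what that actor is.
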(event Custom|GatherInRadius
  (bind _returnvalue (Transformation|GetActorLocation))
  (bind (_outhits _returnvalue_2) (Collision|MultiSphereTraceForObjects _returnvalue (+ _returnvalue (Variables|Default|GetEndRadius)) (Variables|Default|GetSphereRadius) (Utilities|Array|MakeArray "ObjectTypeQuery11") false 0 "None"))
  (if _returnvalue_2
    (for _array_element _outhits
      (Class|PrimalItem|AddNewItem (Variables|Default|GetItemToPickup) (Variables|Default|GetGiveToInventory) false false 1.0 false 1 false 0.0 false)
      (Actor|DestroyActor (.HitActor (Collision|BreakHitResult _array_element))))))

(event EventBeginPlay
  (Utilities|Time|SetTimerbyFunctionName 0 "GatherInRadius" 5.0 true))

(fn ConstructionScript
  (|CallParentFunction))